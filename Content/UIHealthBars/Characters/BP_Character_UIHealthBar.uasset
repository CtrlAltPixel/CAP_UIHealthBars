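; Character Blueprint for the UI health bar system that relays replicated health, resource, armour and spell shield stats as update events.
; Each RepNotify broadcasts the matching OnUpdate dispatcher, pairing current and max values for health and resource.
; BeginPlay calls InitCasts, which is empty, and the WB_UnitHUD_Healthbars creation and SetWidget nodes are disconnected, so no widget is set up here.
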(event `self.ReceiveBeginPlay`
  (`self.InitCasts`))

(fn `InitCasts`)

(fn `OnRep_Armour`
  (`self.OnUpdateArmour` (`self.Armour`)))

(fn `OnRep_CurrentHealth`
  (`self.OnUpdateHealth` (`self.CurrentHealth`) (`self.MaxHealth`)))

(fn `OnRep_CurrentResource`
  (`self.OnUpdateResource` (`self.CurrentResource`) (`self.MaxResource`)))

(fn `OnRep_MaxHealth`
  (`self.OnUpdateHealth` (`self.CurrentHealth`) (`self.MaxHealth`)))

(fn `OnRep_MaxResource`
  (`self.OnUpdateResource` (`self.CurrentResource`) (`self.MaxResource`)))

(fn `OnRep_SpellShield`
  (`self.OnUpdateSpellShield` (`self.SpellShield`)))

(fn `UserConstructionScript`)