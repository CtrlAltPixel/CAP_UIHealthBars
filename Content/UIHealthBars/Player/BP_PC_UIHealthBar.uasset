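; Player controller for the UI health bar feature that caches the camera pawn and HUD and can spawn a health-bar character.
; On BeginPlay, only the local controller runs InitCasts to store the BP_Pawn_Camera and BP_HUD_UIHealthBar references.
; SERVER_SpawnUnit spawns a BP_Character_UIHealthBar at the camera pawn's transform and stores it, relying on that locally cached pawn reference being valid.
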(event `self.ReceiveBeginPlay`
  (if (`self.IsLocalPlayerController`)
    (`self.InitCasts`)))

(event `SERVER_SpawnUnit`
  (bind _as_bp_pawn_camera (`self.As BP Pawn Camera`)
    (:`then`
      (bind _returnvalue (`|SpawnActorFromClass` "/Game/UIHealthBars/Characters/BP_Character_UIHealthBar.BP_Character_UIHealthBar_C" (`self.GetTransform` _as_bp_pawn_camera) "Undefined" "MultiplyWithRoot" null null))
      (set `self.AsCharacterUIHealth` _returnvalue))
    (:`else`)))

(fn `InitCasts`
  (bind _asbp_pawn_camera (cast `/Game/UIHealthBars/Camera/BP_Pawn_Camera` (`self.K2_GetPawn`)))
  (set `self.As BP Pawn Camera` _asbp_pawn_camera)
  (bind _asbp_hud_uihealth_bar (cast `/Game/UIHealthBars/HUD/BP_HUD_UIHealthBar` (`self.GetHUD`)))
  (set `self.As BP HUD UIHealth Bar` _asbp_hud_uihealth_bar))

(fn `UserConstructionScript`)