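; Player controller for the UI health bar feature that spawns the player's unit and links it to the HUD.
; On BeginPlay for the local controller, it adds the default Enhanced Input mapping context and caches the camera pawn and HUD.
; A server-named event then spawns a BP_Character_UIHealthBar at the camera pawn's root transform.
; The spawned character is stored and passed to the HUD as its actor reference.
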(event `self.ReceiveBeginPlay`
  (if (`self.IsLocalPlayerController`)
    (`EnhancedInputSubsystemInterface.AddMappingContext` (pcsubsystem `EnhancedInputLocalPlayerSubsystem` (`GameplayStatics.GetPlayerController` 0)) "/Game/UIHealthBars/Input/IMC_Default.IMC_Default" 0 (struct))
    (`self.InitCasts`)
    (`self.SERVER_SpawnUnit`)))

(event `SERVER_SpawnUnit`
  (bind _as_bp_pawn_camera (`self.As BP Pawn Camera`)
    (:`then`
      (bind _returnvalue (`|SpawnActorFromClass` "/Game/UIHealthBars/Characters/BP_Character_UIHealthBar.BP_Character_UIHealthBar_C" (`SceneComponent.K2_GetComponentToWorld` (`/Game/UIHealthBars/Camera/BP_Pawn_Camera.DefaultSceneRoot` _as_bp_pawn_camera)) "Undefined" "MultiplyWithRoot" null null))
      (set `self.AsCharacterUIHealth` _returnvalue)
      (`self.UpdateUI`))
    (:`else`)))

(event `UpdateUI`
  (bind _as_bp_hud_uihealth_bar (`self.As BP HUD UIHealth Bar`)
    (:`then`
      (`/Game/UIHealthBars/UI/HUD/BP_HUD_UIHealthBar.UpdateActorRef` _as_bp_hud_uihealth_bar (`self.AsCharacterUIHealth`)))
    (:`else`)))

(fn `InitCasts`
  (bind _asbp_pawn_camera (cast `/Game/UIHealthBars/Camera/BP_Pawn_Camera` (`self.K2_GetPawn`)))
  (set `self.As BP Pawn Camera` _asbp_pawn_camera)
  (bind _asbp_hud_uihealth_bar (cast `/Game/UIHealthBars/UI/HUD/BP_HUD_UIHealthBar` (`self.GetHUD`)))
  (set `self.As BP HUD UIHealth Bar` _asbp_hud_uihealth_bar))

(fn `UserConstructionScript`)